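; Interactable wall Blueprint, named as destructible, that responds to players able to cast the Reflect/Refract ability.
; Selectable tints the Cube yellow via SelectColor while selected by such a player, otherwise restoring the default color that the construction script applies.
; Action changes that player's AbilitiesCastingState under the same ability check; no destruction logic lives in this Blueprint.
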(event `/Game/MHarris/Data/I_Selectable_BP.Selectable`
  (params (Selected :type Boolean) (Player :type "/Game/Core/Blueprints/Player/PlayerPawn Object Reference"))
  (`/Engine/EditorBlueprintResources/StandardMacros.IsValid` Player
    (:`Is Valid`
      (if (and Selected (`/Game/Core/Blueprints/Player/PlayerPawn.CanCastReflectRefract` Player))
        (`self.SelectColor` (struct :`R` 0.859375 :`G` 0.851073 :`B` 0.068721 :`A` 1.0))
        (else
          (`self.SelectColor` (`self.DwfaultColor`)))))))

(event `/Game/MHarris/Data/I_Selectable_BP.Action`
  (params (ThePlayer :type "/Game/Core/Blueprints/Player/PlayerPawn Object Reference"))
  (if (`/Game/Core/Blueprints/Player/PlayerPawn.CanCastReflectRefract` ThePlayer)
    (set `/Game/Core/Blueprints/Player/PlayerPawn.AbilitiesCastingState` "NewEnumerator1" ThePlayer)))

(fn `SelectColor`
  (params (Color :type "LinearColor Structure"))
  (`MeshComponent.SetVectorParameterValueOnMaterials` (`self.Cube`) "Color" (`KismetMathLibrary.Conv_LinearColorToVector` Color)))

(fn `UserConstructionScript`
  (`parent.UserConstructionScript`)
  (`MeshComponent.SetVectorParameterValueOnMaterials` (`self.Cube`) "Color" (`KismetMathLibrary.Conv_LinearColorToVector` (`self.DwfaultColor`))))