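; Interactable is a tile-based actor with an empty InteractEvent and events to move, shoot or reflect between tiles.
; MovetoTile and ShoottoTile lerp the actor to enterable tiles on separate timelines.
; ReflecttoTile skips the CanEnter check and lerps a supplied projectile from this actor's current tile with an added height arc.
; All three finish by calling OnExit, updating this actor's tile references and calling OnEntered.
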(event `/Game/Core/Blueprints/Interfaces/I_Interactable.Interact Event`
  (params (Player :type "/Game/Core/Blueprints/Player/PlayerPawn Object Reference")))

(event `/Game/Core/Blueprints/Interfaces/I_Moveable.MoveToTile`
  (params (`Target Tile` :type "/Game/Core/Blueprints/Tile_Assets/Tile Object Reference"))
  ;[1 1 1] If target tile is valid and is enterable, assign it to Target Tile variable
  (`/Engine/EditorBlueprintResources/StandardMacros.IsValid` `Target Tile`
    (:`Is Valid`
      (if (`/Game/Core/Blueprints/Tile_Assets/Tile.Can Enter` `Target Tile`)
        (set `self.Target Tile` `Target Tile`)
        ;[1 1 1] Timeline and Lerp for smooth movement instead of visually teleporting
        (bind (_direction _move_progress) (`Timeline|Timeline_0` :!via `PlayFromStart`)
          (:`Update`
            ;[1 1 1] This actually moves the actor
            (`self.K2_SetActorLocation` (`KismetMathLibrary.VLerp` (`self.K2_GetActorLocation` (`self.Current Tile`)) (`self.K2_GetActorLocation` `Target Tile`) _move_progress)))
          (:`Finished`
            ;[1 1 1] Call On Exit even for current tile
            (`/Game/Core/Blueprints/Tile_Assets/Tile.On Exit` (`self.Current Tile`) null (`self.Target Tile`) self)
            ;[1 1 1] Assign Current Tile as Previous Tile and Target Tile as Current Tile
            (set `self.Previous Tile` (`self.Current Tile`))
            (set `self.Current Tile` (`self.Target Tile`))
            ;[1 1 1] Empty our Target Tile variable
            (set `self.Target Tile` null)
            ;[1 1 1] Call On Entered event for new Current Tile
            (`/Game/Core/Blueprints/Tile_Assets/Tile.On Entered` (`self.Current Tile`) null (`self.Previous Tile`) self)))))))

(event `/Game/Core/Blueprints/Interfaces/I_Moveable.ReflectToTile`
  (params (`Target Tile` :type "/Game/Core/Blueprints/Tile_Assets/Tile Object Reference") (Projectile :type "/Game/MHarris/Interactable_Projectile Object Reference"))
  ;[1 1 1] If target tile is valid and is enterable, assign it to Target Tile variable
  (`/Engine/EditorBlueprintResources/StandardMacros.IsValid` `Target Tile`
    (:`Is Valid`
      (set `self.ProjectileLocation` (`self.K2_GetActorLocation` Projectile))
      (if true
        (set `self.Target Tile` `Target Tile`)
        ;[1 1 1] Timeline and Lerp for smooth movement instead of visually teleporting
        (bind (_direction _move_progress _alphaarch) (`Timeline|ArchReflect` :!via `PlayFromStart`)
          (:`Update`
            ;[1 1 1] This actually moves the actor
            (`self.K2_SetActorLocation` Projectile (+ (`KismetMathLibrary.VLerp` (`self.K2_GetActorLocation` (`self.Current Tile`)) (`self.K2_GetActorLocation` `Target Tile`) _move_progress) (`KismetMathLibrary.MakeVector` 0.0 0.0 (`KismetMathLibrary.Lerp` 0.0 50.0 _alphaarch))) false false))
          (:`Finished`
            ;[1 1 1] Call On Exit even for current tile
            (`/Game/Core/Blueprints/Tile_Assets/Tile.On Exit` (`self.Current Tile`) null (`self.Target Tile`) self)
            ;[1 1 1] Assign Current Tile as Previous Tile and Target Tile as Current Tile
            (set `self.Previous Tile` (`self.Current Tile`))
            (set `self.Current Tile` (`self.Target Tile`))
            ;[1 1 1] Empty our Target Tile variable
            (set `self.Target Tile` null)
            ;[1 1 1] Call On Entered event for new Current Tile
            (`/Game/Core/Blueprints/Tile_Assets/Tile.On Entered` (`self.Current Tile`) null (`self.Previous Tile`) self)))))))

(event `/Game/Core/Blueprints/Interfaces/I_Moveable.ShootToTile`
  (params (`Target Tile` :type "/Game/Core/Blueprints/Tile_Assets/Tile Object Reference"))
  ;[1 1 1] If target tile is valid and is enterable, assign it to Target Tile variable
  (`/Engine/EditorBlueprintResources/StandardMacros.IsValid` `Target Tile`
    (:`Is Valid`
      (if (`/Game/Core/Blueprints/Tile_Assets/Tile.Can Enter` `Target Tile`)
        (set `self.Target Tile` `Target Tile`)
        ;[1 1 1] Timeline and Lerp for smooth movement instead of visually teleporting
        (bind (_direction _move_progress) (`Timeline|T_Shooting` :!via `PlayFromStart`)
          (:`Update`
            ;[1 1 1] This actually moves the actor
            (`self.K2_SetActorLocation` (`KismetMathLibrary.VLerp` (`self.K2_GetActorLocation` (`self.Current Tile`)) (`self.K2_GetActorLocation` `Target Tile`) _move_progress)))
          (:`Finished`
            ;[1 1 1] Call On Exit even for current tile
            (`/Game/Core/Blueprints/Tile_Assets/Tile.On Exit` (`self.Current Tile`) null (`self.Target Tile`) self)
            ;[1 1 1] Assign Current Tile as Previous Tile and Target Tile as Current Tile
            (set `self.Previous Tile` (`self.Current Tile`))
            (set `self.Current Tile` (`self.Target Tile`))
            ;[1 1 1] Empty our Target Tile variable
            (set `self.Target Tile` null)
            ;[1 1 1] Call On Entered event for new Current Tile
            (`/Game/Core/Blueprints/Tile_Assets/Tile.On Entered` (`self.Current Tile`) null (`self.Previous Tile`) self)))))))

(fn `UserConstructionScript`)