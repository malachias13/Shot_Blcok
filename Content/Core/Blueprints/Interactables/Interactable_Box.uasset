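; Pushable box interactable for tile-based movement that a player shoves one tile away from themselves at a stamina cost.
; On InteractEvent it checks stamina and that the player stands on another tile, then uses TileIsNeighbor's opposite direction to find the destination.
; If that neighbor exists and can be entered, the box moves there and spends stamina, toggling player interaction around the move.
; Failed checks only print a message.
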(event `/Game/Core/Blueprints/Interfaces/I_Interactable.Interact Event`
  (params (Player :type "/Game/Core/Blueprints/Player/PlayerPawn Object Reference"))
  (bind _player (`self.Player`))
  (bind _player_2 (`self.Player`))
  (bind _output_get (set `self.Player` Player))
  (if (and (>= (`/Game/Core/Blueprints/Player/PlayerPawn.Stamina` _player_2) (`self.StaminaRequired`)) (!= (`/Game/Core/Blueprints/Player/PlayerPawn.Current Tile` _player_2) (`self.Current Tile`)))
    ;[1 1 1] Is the player's current tile a neighbor? If so, grab the opposite direction to determine tile to move to
    (bind _direction (`/Game/Core/Blueprints/Tile_Assets/Tile.Tile Is Neighbor?` (`self.Current Tile`) (`/Game/Core/Blueprints/Player/PlayerPawn.Current Tile` _output_get)))
    (bind (_value _returnvalue) (`BlueprintMapLibrary.Map_Find` (`/Game/Core/Blueprints/Tile_Assets/Tile.Neighbors` (`self.Current Tile`)) (`/Game/Core/Blueprints/Tile_Assets/Direction.OppositeDirection` _direction)))
    ;[1 1 1] Checking if Tile exists and can be entered
    (if (and (`/Game/Core/Blueprints/Tile_Assets/Tile.Can Enter` _value) _returnvalue)
      ;[1 1 1] Toggle Interact, moving interactable to tile, and using stamina
      (`/Game/Core/Blueprints/Player/PlayerPawn.ToggleInteract` (`self.Player`) false)
      (`self.MoveToTile` _value)
      (message `/Game/Core/Blueprints/Interfaces/I_Player.Stamina Use` _player (`self.StaminaRequired`))
      (`/Game/Core/Blueprints/Player/PlayerPawn.ToggleInteract` _player true)
      (else
        (`KismetSystemLibrary.PrintString` "Can't move it there!")))
    (else
      (`KismetSystemLibrary.PrintString` "Not Enough Stamina!"))))

(fn `UserConstructionScript`
  (`parent.UserConstructionScript`))