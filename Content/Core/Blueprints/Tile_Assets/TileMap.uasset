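; Tile map actor that builds and owns a rectangular grid of tiles and sets up the camera and player at BeginPlay.
; GenerateMap destroys old tiles and their interactables, spawns attached border and fill tiles, then has each find its neighbors.
; Helpers convert coords to flat array indices for lookup and replacement.
; BeginPlay moves the player pawn to the spawn tile, initializes its tile and direction, and makes that tile non-enterable.
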(event `self.ReceiveBeginPlay`
  (bind _returnvalue (`GameplayStatics.GetPlayerPawn` 0))
  ;[1 1 1] Set Main Camera
  (`PlayerController.SetViewTargetWithBlend` (`GameplayStatics.GetPlayerController` 0) (`self.Camera Actor`) 0.0 "VTBlend_Linear" 0.0 false)
  ;[1 1 1] Spawn Player
  (`self.K2_SetActorLocation` _returnvalue (`self.K2_GetActorLocation` (`self.Player Spawn Tile`)) false false)
  (`self.K2_SetActorRotation` _returnvalue (`/Game/Core/Blueprints/Tile_Assets/Direction.Rotation` (`self.Player Spawn Direction`)) false)
  ;[1 1 1] Initialize Variables on Player, Make Player Spawn Tile Not Enterable
  (bind _asplayer_pawn (cast `/Game/Core/Blueprints/Player/PlayerPawn` _returnvalue))
  (set `/Game/Core/Blueprints/Player/PlayerPawn.Current Tile` (`self.Player Spawn Tile`) _asplayer_pawn)
  (set `/Game/Core/Blueprints/Player/PlayerPawn.Current Direction` (`self.Player Spawn Direction`) _asplayer_pawn)
  (set `/Game/Core/Blueprints/Tile_Assets/Tile.Can Enter` false (`self.Player Spawn Tile`)))

(fn `CoordToIndex`
  (params (Coord :type "/Game/Core/Blueprints/Tile_Assets/Coord Structure"))
  (returns (Index :type Integer))
  (return (+ Coord_X_5_6F435FC24D9202AE27D58A9D538EE86B (* Coord_Y_7_1CB6DBA146075157CAA02385B7A6DC31 (`self.Width`)))))

(fn `GenerateMap`
  (for _array_element (`self.Tiles`)
    (`/Engine/EditorBlueprintResources/StandardMacros.IsValid` _array_element
      (:`Is Valid`
        (bind _currentinteractableactor (`/Game/Core/Blueprints/Tile_Assets/Tile.CurrentInteractableActor` _array_element))
        ;[1 1 1] If current obstacle is NOT null, destroy it
        (if (!= _currentinteractableactor null)
          (`self.K2_DestroyActor` _currentinteractableactor))
        ;[1 1 1] Destroy Tile
        (`self.K2_DestroyActor` _array_element))))
  (`KismetArrayLibrary.Array_Clear` (`self.Tiles`))
  (for _index (range (`self.Height`))
    (for _index_2 (range (`self.Width`))
      (bind _returnvalue (select `bool` (`self.IsCoordOnBorder` (make `/Game/Core/Blueprints/Tile_Assets/Coord` _index_2 _index)) :`false` (`self.Fill Tile Type`) :`true` (`self.Border Tile Type`)))
      (bind _returnvalue_2 (`|SpawnActorFromClass` :`Class` _returnvalue :`SpawnTransform` (`KismetMathLibrary.MakeTransform` (`KismetMathLibrary.MakeVector` (* _index 100.0) (* _index_2 100.0))) :`CollisionHandlingOverride` "Undefined" :`TransformScaleMethod` "OverrideRootScale" :`Coord` (make `/Game/Core/Blueprints/Tile_Assets/Coord` _index_2 _index) :`Tile Map` self :`New Tile Type` _returnvalue :`NewInteractableType` null :`Instigator` null))
      (`KismetArrayLibrary.Array_Add` (`self.Tiles`) _returnvalue_2)
      (`self.K2_AttachToActor` _returnvalue_2 self "None" "KeepWorld" "KeepWorld" "KeepWorld" true)))
  (for _array_element_2 (`self.Tiles`)
    (`/Game/Core/Blueprints/Tile_Assets/Tile.FindNeighbors` _array_element_2)))

(fn `GetTileAtCoord`
  (params (Coord :type "/Game/Core/Blueprints/Tile_Assets/Coord Structure"))
  (returns (Tile :type "/Game/Core/Blueprints/Tile_Assets/Tile Object Reference"))
  (return (`|GetArrayItem` (`self.Tiles`) (`self.CoordToIndex` Coord))))

(fn `IndexToCoord`
  (params (Index :type Integer))
  (returns (Coord :type "/Game/Core/Blueprints/Tile_Assets/Coord Structure"))
  (bind _width (`self.Width`))
  (return (make `/Game/Core/Blueprints/Tile_Assets/Coord` (mod Index _width) (/ Index _width))))

(fn `IsCoordInRange`
  (params (Coord :type "/Game/Core/Blueprints/Tile_Assets/Coord Structure"))
  (returns (`Is In Range?` :type Boolean))
  (return (not (or (< Coord_X_5_6F435FC24D9202AE27D58A9D538EE86B 0) (< Coord_Y_7_1CB6DBA146075157CAA02385B7A6DC31 0) (>= Coord_X_5_6F435FC24D9202AE27D58A9D538EE86B (`self.Width`)) (>= Coord_Y_7_1CB6DBA146075157CAA02385B7A6DC31 (`self.Height`))))))

(fn `IsCoordOnBorder`
  (params (Coord :type "/Game/Core/Blueprints/Tile_Assets/Coord Structure"))
  (returns (IsOnBorder :type Boolean))
  (return (or (== Coord_X_5_6F435FC24D9202AE27D58A9D538EE86B 0) (== Coord_X_5_6F435FC24D9202AE27D58A9D538EE86B (- (`self.Width`) 1)) (== Coord_Y_7_1CB6DBA146075157CAA02385B7A6DC31 0) (== Coord_Y_7_1CB6DBA146075157CAA02385B7A6DC31 (- (`self.Height`) 1)))))

(fn `Replace Tile`
  (params (`New Tile` :type "/Game/Core/Blueprints/Tile_Assets/Tile Object Reference"))
  (`KismetArrayLibrary.Array_Set` (`self.Tiles`) (`self.CoordToIndex` (`/Game/Core/Blueprints/Tile_Assets/Tile.Coord` `New Tile`)) `New Tile`))

(fn `SetSpawnTile`
  (params (`Tile To Set` :type "/Game/Core/Blueprints/Tile_Assets/Tile Object Reference"))
  (set `self.Player Spawn Tile` `Tile To Set`))

(fn `UserConstructionScript`)