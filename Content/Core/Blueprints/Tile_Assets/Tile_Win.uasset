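; Tile_Win is the goal tile that celebrates a win and moves the game to another level.
; It extends the parent tile's OnEntered event and, for a valid player, disables input on the first player pawn, plays a cheering sound and activates a confetti particle system.
; A delay equal to the sound's duration holds the celebration before opening the level named by NameOfLevelToLoad.
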(event `self.On Entered`
  (params (Player :type "/Game/Core/Blueprints/Player/PlayerPawn Object Reference") (`Previous Tile` :type "/Game/Core/Blueprints/Tile_Assets/Tile Object Reference") (Interactable :type "/Game/Core/Blueprints/Interactables/Interactable Object Reference"))
  (`parent.On Entered` Player `Previous Tile` Interactable)
  (if (`KismetSystemLibrary.IsValid` Player)
    (`self.DisableInput` (`GameplayStatics.GetPlayerPawn` 0) null)
    ;[1 1 1] Make and play sound
    (bind _returnvalue (`GameplayStatics.SpawnSound2D` "/Game/Core/Sound/kids_cheering.kids_cheering" 1.0 1.0 0.0 null))
    (`AudioComponent.Play` _returnvalue 0.0)
    ;[1 1 1] Play Particle System
    (`ActorComponent.Activate` (`self.ConfettiSystem`) true)
    (`KismetSystemLibrary.Delay` (`SoundBase.Duration` (`AudioComponent.Sound` _returnvalue)))
    (`GameplayStatics.OpenLevel` (`KismetStringLibrary.Conv_StringToName` (`self.nameOfLevelToLoad`)))))

(fn `UserConstructionScript`
  (`parent.UserConstructionScript`))