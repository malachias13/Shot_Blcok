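; Tile_Message is a tile Blueprint that prints a debug message when something enters it.
; On OnEntered it calls the parent handler, then prints the object name of the entering Player, or of the Interactable if no valid Player is given.
; Its CanPlayerEnter override always returns true, so it never blocks player movement.
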(event `self.On Entered`
  (params (Player :type "/Game/Core/Blueprints/Player/PlayerPawn Object Reference") (`Previous Tile` :type "/Game/Core/Blueprints/Tile_Assets/Tile Object Reference") (Interactable :type "/Game/Core/Blueprints/Interactables/Interactable Object Reference"))
  (`parent.On Entered` Player `Previous Tile` Interactable)
  (if (`KismetSystemLibrary.IsValid` Player)
    (set `self.DebugMessage` (`KismetSystemLibrary.GetObjectName` Player))
    (`KismetSystemLibrary.PrintString` (`self.DebugMessage`) :!label _label)
    (elif (`KismetSystemLibrary.IsValid` Interactable)
      (set `self.DebugMessage` (`KismetSystemLibrary.GetObjectName` Interactable))
      (goto _label))))

(fn `Can Player Enter`
  (params (Player :type "/Game/Core/Blueprints/Player/PlayerPawn Object Reference") (From :type "/Game/Core/Blueprints/Tile_Assets/Tile Object Reference"))
  (returns (`Can Enter` :type Boolean))
  (return true))

(fn `UserConstructionScript`
  (`parent.UserConstructionScript`))