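; Grid tile actor that links to its four orthogonal neighbors through its TileMap and tracks whether it can be entered.
; Entering blocks the tile and records any interactable; exiting frees it.
; UpdateTileType spawns or clears interactables, or replaces itself with a new tile class, relinking neighbors and the map.
; TileIsNeighbor returns an adjacent tile's direction, skipping a stray None direction seen only in builds.
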(event `self.ReceiveBeginPlay`
  (`self.FindNeighbors`))

(event `On Entered`
  (params (Player :type "/Game/Core/Blueprints/Player/PlayerPawn Object Reference") (`Previous Tile` :type "/Game/Core/Blueprints/Tile_Assets/Tile Object Reference") (Interactable :type "/Game/Core/Blueprints/Interactables/Interactable Object Reference"))
  (bind _returnvalue (`KismetSystemLibrary.IsValid` Interactable))
  ;[1 1 1] Is either player or interactable valid?
  (if (or (`KismetSystemLibrary.IsValid` Player) _returnvalue)
    (set `self.Can Enter` false)
    (if _returnvalue
      (set `self.NewInteractableType` (`GameplayStatics.GetObjectClass` Interactable))
      (set `self.CurrentInteractableActor` Interactable))
    (else
      (`KismetSystemLibrary.PrintString` "Invalid Player or Interactable"))))

(event `On Exit`
  (params (Player :type "/Game/Core/Blueprints/Player/PlayerPawn Object Reference") (`Target Tile` :type "/Game/Core/Blueprints/Tile_Assets/Tile Object Reference") (Interactable :type "/Game/Core/Blueprints/Interactables/Interactable Object Reference"))
  (bind _returnvalue (`KismetSystemLibrary.IsValid` Interactable))
  ;[1 1 1] Is either player or interactable valid?
  (if (or (`KismetSystemLibrary.IsValid` Player) _returnvalue)
    (set `self.Can Enter` true)
    ;[1 1 1] If an interactable has left, empty interactable variables
    (if _returnvalue
      (set `self.NewInteractableType` null)
      (set `self.CurrentInteractableActor` null))
    (else
      (`KismetSystemLibrary.PrintString` "Invalid Player or Interactable"))))

(fn `Can Player Enter`
  (params (Player :type "/Game/Core/Blueprints/Player/PlayerPawn Object Reference") (From :type "/Game/Core/Blueprints/Tile_Assets/Tile Object Reference"))
  (returns (`Can Enter` :type Boolean))
  (return (`self.Can Enter`)))

(fn `FindNeighbors`
  (bind (_coord_x _coord_y) (break `/Game/Core/Blueprints/Tile_Assets/Coord` (`self.Coord`)))
  (for _array_element (`|MakeArray` "/Game/Core/Blueprints/Tile_Assets/Up.Up" "/Game/Core/Blueprints/Tile_Assets/Down.Down" "/Game/Core/Blueprints/Tile_Assets/Left.Left" "/Game/Core/Blueprints/Tile_Assets/Right.Right" :!type "/Game/Core/Blueprints/Tile_Assets/Direction Object Reference")
    (bind (_delta_x _delta_y) (break `/Game/Core/Blueprints/Tile_Assets/Coord` (`/Game/Core/Blueprints/Tile_Assets/Direction.Delta` _array_element)))
    (bind _returnvalue (+ _delta_x _coord_x))
    (bind _returnvalue_2 (+ _delta_y _coord_y))
    (if (`/Game/Core/Blueprints/Tile_Assets/TileMap.IsCoordInRange` (`self.Tile Map`) (make `/Game/Core/Blueprints/Tile_Assets/Coord` _returnvalue _returnvalue_2))
      (bind _tile (`/Game/Core/Blueprints/Tile_Assets/TileMap.GetTileAtCoord` (`self.Tile Map`) (make `/Game/Core/Blueprints/Tile_Assets/Coord` _returnvalue _returnvalue_2)))
      (`/Engine/EditorBlueprintResources/StandardMacros.IsValid` _tile
        (:`Is Valid`
          (`BlueprintMapLibrary.Map_Add` (`self.Neighbors`) _array_element _tile))))))

(fn `Set Neighbor`
  (params (Direction :type "/Game/Core/Blueprints/Tile_Assets/Direction Object Reference") (`New Neighbor` :type "/Game/Core/Blueprints/Tile_Assets/Tile Object Reference"))
  (`BlueprintMapLibrary.Map_Add` (`self.Neighbors`) Direction `New Neighbor`))

(fn `SetAsSpawnTile`
  (`/Game/Core/Blueprints/Tile_Assets/TileMap.SetSpawnTile` (`self.Tile Map`) self))

(fn `Tile Is Neighbor?`
  (params (Tile :type "/Game/Core/Blueprints/Tile_Assets/Tile Object Reference"))
  (returns (Direction :type "/Game/Core/Blueprints/Tile_Assets/Direction Object Reference"))
  (locals (CheckNeighborTile :type "/Game/Core/Blueprints/Tile_Assets/Tile Object Reference"))
  ;[1 1 1] Assign Tile being checked as local variable
  (set `local.CheckNeighborTile` Tile)
  ;[1 1 1] Step through each Neighboring tile
  (bind _values (`BlueprintMapLibrary.Map_Values` (`self.Neighbors`)))
  (for _array_element _values
    ;[1 1 1] Is current neighbor equal to tile being checked?
    (if (== (`local.CheckNeighborTile`) _array_element)
      ;[1 1 1] Step through each direction of neighbors
      (bind _keys (`BlueprintMapLibrary.Map_Keys` (`self.Neighbors`)))
      (for _array_element_2 _keys
        ;[1 1 1] If the current direction's tile matches the tile being checked, the tile is a neighbor in that direction, return that direction information
        (if (and (!= _array_element_2 null) (== (`local.CheckNeighborTile`) (`BlueprintMapLibrary.Map_Find` (`self.Neighbors`) _array_element_2)))
          (return _array_element_2))))))

(fn `UpdateTileType`
  (bind _tile_map (`self.Tile Map`))
  (bind _new_tile_type (`self.New Tile Type`))
  (bind _currentinteractableactor (`self.CurrentInteractableActor`))
  (bind _new_tile_type_2 (`self.New Tile Type`))
  ;[1 1 1] Spawn new obstacle if it's selected, delete old one
  (if (== (`self.NewInteractableType`) null)
    ;[1 1 1] If there is a current valid obstacle, destroy it. Empty the variable either way
    (`/Engine/EditorBlueprintResources/StandardMacros.IsValid` (`self.CurrentInteractableActor`)
      (:`Is Valid`
        (`self.K2_DestroyActor` (`self.CurrentInteractableActor`)))
      (:`Is Not Valid`
        _))
    (set `self.CurrentInteractableActor` null)
    (if (and (`KismetSystemLibrary.IsValidClass` _new_tile_type) (!= _new_tile_type (`GameplayStatics.GetObjectClass` self)))
      ;[1 1 1] Spawn new tile from type
      (bind _returnvalue (`|SpawnActorFromClass` _new_tile_type_2 (`self.GetTransform`) "AlwaysSpawn" "OverrideRootScale" null (`self.Coord`) (`self.Neighbors`) (`self.Tile Map`) _new_tile_type_2 (`self.NewInteractableType`) null))
      ;[1 1 1] Step through each direction and add neighboring tiles
      (bind _keys (`BlueprintMapLibrary.Map_Keys` (`self.Neighbors`)))
      (for _array_element _keys
        (bind _value (`BlueprintMapLibrary.Map_Find` (`self.Neighbors`) _array_element))
        (`/Engine/EditorBlueprintResources/StandardMacros.IsValid` _value
          (:`Is Valid`
            (`self.Set Neighbor` _value (`/Game/Core/Blueprints/Tile_Assets/Direction.OppositeDirection` _array_element) _returnvalue))))
      ;[1 1 1] Replace the tile in the tile map
      (`/Game/Core/Blueprints/Tile_Assets/TileMap.Replace Tile` _tile_map _returnvalue)
      (`self.K2_AttachToActor` _returnvalue _tile_map "None" "KeepWorld" "KeepWorld" "KeepWorld" true)
      (`self.K2_DestroyActor`)
      (else
        (set `self.Can Enter` true)))
    (else
      (bind _returnvalue_2 (`|SpawnActorFromClass` (`self.NewInteractableType`) (`self.GetTransform`) "AlwaysSpawn" "OverrideRootScale" null 0.0 self null))
      (if (and (!= _returnvalue_2 null) (!= _currentinteractableactor null))
        (`self.K2_DestroyActor` _currentinteractableactor))
      (set `self.CurrentInteractableActor` _returnvalue_2)
      (set `self.Can Enter` false))))

(fn `UserConstructionScript`)