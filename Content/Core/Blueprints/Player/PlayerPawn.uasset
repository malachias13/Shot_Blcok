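; Player pawn for grid-based movement, with stamina, HUD and debug widgets, and interaction with the facing tile's actor.
; Directional input looks up the current tile's neighbor, turns the pawn and lerps it there on a Timeline, then fires tile exit and enter events.
; Interact messages the facing tile's interactable, passing the pawn.
; Stamina use and clamped refill adjust the pool, while Space triggers an action bar dispatch.
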(event `self.ReceiveBeginPlay`
  (set `self.CanInteract` true)
  (set `self.Stamina` (`self.MaxStamina`))
  (bind _returnvalue (`|CreateWidget` "/Game/Core/UI/Blueprints/PlayerHUDWidget.PlayerHUDWidget_C"))
  (`UserWidget.AddToViewport` _returnvalue 0)
  (bind _returnvalue_2 (`|CreateWidget` "/Game/Core/UI/Blueprints/UI_Debug.UI_Debug_C"))
  (`UserWidget.AddToViewport` _returnvalue_2 100))

(event `InputAction|Move Forward`
  (params (Key :type "Key Structure"))
  ;[1 1 1] Input Events
  (:`Pressed`
    (`self.Player Movement` "/Game/Core/Blueprints/Tile_Assets/Up.Up")))

(event `InputAction|Escape`
  (params (Key :type "Key Structure"))
  ;[1 1 1] Input Events
  (:`Pressed`
    (`KismetSystemLibrary.QuitGame` null "Quit")))

(event `InputAction|Move Backward`
  (params (Key :type "Key Structure"))
  ;[1 1 1] Input Events
  (:`Pressed`
    (`self.Player Movement` "/Game/Core/Blueprints/Tile_Assets/Down.Down")))

(event `InputAction|Refill Stamina Debug`
  (params (Key :type "Key Structure"))
  ;[1 1 1] Input Events
  (:`Pressed`
    (`self.Refill Stamina` (`self.MaxStamina`))))

(event `InputAction|Move Right`
  (params (Key :type "Key Structure"))
  ;[1 1 1] Input Events
  (:`Pressed`
    (`self.Player Movement` "/Game/Core/Blueprints/Tile_Assets/Right.Right")))

(event `InputAction|Move Left`
  (params (Key :type "Key Structure"))
  ;[1 1 1] Input Events
  (:`Pressed`
    (`self.Player Movement` "/Game/Core/Blueprints/Tile_Assets/Left.Left")))

(event `InputAction|Interact`
  (params (Key :type "Key Structure"))
  ;[1 1 1] Input Events
  (:`Pressed`
    (`self.Player Interact`)))

(event `InputAction|Space Bar`
  (params (Key :type "Key Structure"))
  ;[1 1 1] Input Events
  (:`Pressed`
    (`self.ActionBarDispatch`)))

(event `/Game/Core/Blueprints/Interfaces/I_Moveable.MoveToTile`
  (params (`Target Tile` :type "/Game/Core/Blueprints/Tile_Assets/Tile Object Reference"))
  ;[1 1 1] Move To Tile
  ;[1 1 1] If target tile is valid and is enterable, assign it to Target Tile variable
  (`/Engine/EditorBlueprintResources/StandardMacros.IsValid` `Target Tile`
    (:`Is Valid`
      (if (`/Game/Core/Blueprints/Tile_Assets/Tile.Can Enter` `Target Tile`)
        (set `self.Target Tile` `Target Tile`)
        ;[1 1 1] Timeline and Lerp for smooth movement instead of visually teleporting
        (bind (_direction _move_progress) (`Timeline|Move Timeline` :!via `PlayFromStart`)
          (:`Update`
            ;[1 1 1] This actually moves the player pawn
            (`self.K2_SetActorLocation` (`KismetMathLibrary.VLerp` (`self.K2_GetActorLocation` (`self.Current Tile`)) (`self.K2_GetActorLocation` `Target Tile`) _move_progress)))
          (:`Finished`
            ;[1 1 1] Call On Exit even for current tile
            (`/Game/Core/Blueprints/Tile_Assets/Tile.On Exit` (`self.Current Tile`) self (`self.Target Tile`) null)
            ;[1 1 1] Assign Current Tile as Previous Tile and Target Tile as Current Tile
            (set `self.Previous Tile` (`self.Current Tile`))
            (set `self.Current Tile` (`self.Target Tile`))
            ;[1 1 1] Empty our Target Tile variable
            (set `self.Target Tile` null)
            ;[1 1 1] Call On Entered event for new Current Tile
            (`/Game/Core/Blueprints/Tile_Assets/Tile.On Entered` (`self.Current Tile`) self (`self.Previous Tile`) null)))))))

(event `Face Direction`
  (params (`Target Direction` :type "/Game/Core/Blueprints/Tile_Assets/Direction Object Reference"))
  ;[1 1 1] Update Face Direction
  (`/Engine/EditorBlueprintResources/StandardMacros.IsValid` `Target Direction`
    (:`Is Valid`
      (set `self.Target Direction` `Target Direction`)
      (`self.K2_SetActorRotation` (`/Game/Core/Blueprints/Tile_Assets/Direction.Rotation` (`self.Target Direction`)))
      (set `self.Current Direction` (`self.Target Direction`))
      (set `self.Target Direction` null))))

(event `/Game/Core/Blueprints/Interfaces/I_Player.Stamina Use`
  (params (`Stamina Requirement` :type "Float (single-precision)"))
  ;[1 1 1] Update Stamina after obstacle interaction
  (set `self.Stamina` (- (`self.Stamina`) `Stamina Requirement`)))

(fn `Player Interact`
  (bind (_value _returnvalue) (`BlueprintMapLibrary.Map_Find` (`/Game/Core/Blueprints/Tile_Assets/Tile.Neighbors` (`self.Current Tile`)) (`self.Current Direction`)))
  (bind _currentinteractableactor (`/Game/Core/Blueprints/Tile_Assets/Tile.CurrentInteractableActor` _value))
  ;[1 1 1] If Tile and Obstacle exist, interact with the Obstacle
  (if _returnvalue
    (if (!= _currentinteractableactor null)
      (message `/Game/Core/Blueprints/Interfaces/I_Interactable.Interact Event` _currentinteractableactor self))))

(fn `Player Movement`
  (params (Direction :type "/Game/Core/Blueprints/Tile_Assets/Direction Object Reference"))
  (locals (MoveDirection :type "/Game/Core/Blueprints/Tile_Assets/Direction Object Reference"))
  (bind _value (`BlueprintMapLibrary.Map_Find` (`/Game/Core/Blueprints/Tile_Assets/Tile.Neighbors` (`self.Current Tile`)) (`local.MoveDirection`)))
  ;[1 1 1] Promote given direction to Move Direction variable
  (set `local.MoveDirection` Direction)
  ;[1 1 1] If Player can move and there is no valid Target Tile
  (if (`self.Can Move`)
    (`/Engine/EditorBlueprintResources/StandardMacros.IsValid` (`self.Target Tile`)
      (:`Is Not Valid`
        ;[1 1 1] Is the tile a valid object?
        (`/Engine/EditorBlueprintResources/StandardMacros.IsValid` _value
          (:`Is Valid`
            ;[1 1 1] Call Move To Tile and Face Direction events
            (`/Game/Core/Blueprints/Interfaces/I_Moveable.MoveToTile` _value)
            (`self.Face Direction` (`local.MoveDirection`)))
          (:`Is Not Valid`
            (`KismetSystemLibrary.PrintString` "Error: Can't locate next tile." true true (`KismetMathLibrary.LinearColor_Red`))))))))

(fn `Refill Stamina`
  (params (AmountToAdd :type "Float (double-precision)"))
  (set `self.Stamina` (`KismetMathLibrary.FClamp` (+ AmountToAdd (`self.Stamina`)) 0.0 (`self.MaxStamina`))))

(fn `ToggleInteract`
  (params (`Interact?` :type Boolean))
  (set `self.CanInteract` `Interact?`))

(fn `UserConstructionScript`)