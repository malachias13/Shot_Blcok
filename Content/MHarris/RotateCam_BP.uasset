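; RotateCam_BP is an unfinished actor meant to orbit a camera around its own location.
; BeginPlay takes the CameraActor from the level's TileMap and stores the actor's location as CenterPoint.
; The rotation logic never runs: Tick is empty and the update chains are disconnected.
; RoatateAroundVec offsets the camera from a center by a radius, but its angle and axis are zero and its rate is unused.
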(event `self.ReceiveBeginPlay`
  (bind _returnvalue (`GameplayStatics.GetActorOfClass` "/Game/Core/Blueprints/Tile_Assets/TileMap.TileMap_C"))
  (set `self.Camera Actor` (`/Game/Core/Blueprints/Tile_Assets/TileMap.Camera Actor` _returnvalue))
  (set `self.CenterPoint` (`self.K2_GetActorLocation`)))

(event `self.ReceiveTick`
  (params (DeltaSeconds :type "Float (single-precision)")))

(fn `RoatateAroundVec`
  (params (Vec :type "Vector Structure") (Radius :type "Float (double-precision)") (RotRate :type "Float (double-precision)") (Angle :type "Float (double-precision)"))
  (returns (Location :type "Vector Structure"))
  (locals (TargetVec :type "Vector Structure") (L_Radius :type "Float (double-precision)") (L_Rate :type "Float (double-precision)"))
  (set `local.TargetVec` Vec)
  (set `local.L_Radius` Radius)
  (set `local.L_Rate` RotRate)
  (`self.K2_SetActorLocation` (`self.Camera Actor`) (+ (`local.TargetVec`) (`KismetMathLibrary.RotateAngleAxis` (`KismetMathLibrary.MakeVector` (`local.L_Radius`)))) false false)
  (return (`local.TargetVec`)))

(fn `UserConstructionScript`)